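; BP_Boss_Trigger is a one-shot trigger volume that starts the Knight boss encounter.
; On BeginPlay it finds the BP_Knight actors in the level and stores them.
; When the player character overlaps the box, the first Knight plays its battle-start montage and the BossIntro level sequence plays.
; It also calls the player's timed overlay hide-then-show function, then destroys itself.
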(event OnComponentBeginOverlap(Box)
  (params (OverlappedComponent :type Primitive%20Component%20Object%20Reference) (OtherActor :type Actor%20Object%20Reference) (OtherComp :type Primitive%20Component%20Object%20Reference) (OtherBodyIndex :type Integer) (bFromSweep :type Boolean) (SweepResult :type Hit%20Result%20Structure%20%28by%20ref%29))
  (bind _asbp_player_character (Utilities|Casting|CastToBP_PlayerCharacter OtherActor))
  (Animation|PlayAnimMontage (Utilities|Array|Get(acopy) (Variables|Default|GetBoss)) "/Game/Blueprints/Enemy/Knight/Animation/AM_Knight_BattleStart.AM_Knight_BattleStart" 1.0 "None")
  (bind _returnvalue (Sequencer|Player|CreateLevelSequencePlayer "/Game/Blueprints/Sequences/BossBattleStartCinema/BossIntro.BossIntro"))
  (Sequencer|Player|Play _returnvalue :!class /Script/MovieScene.MovieSceneSequencePlayer)
  (Default|OverlayHideAfterShow _asbp_player_character 9.0)
  (Actor|DestroyActor))

(event EventBeginPlay
  (bind _outactors (Actor|GetAllActorsOfClass "/Game/Blueprints/Enemy/Knight/BP_Knight.BP_Knight_C"))
  (Variables|Default|SetBoss _outactors))

(event Collision|EventActorBeginOverlap
  (params (OtherActor :type Actor%20Object%20Reference)))

(event EventTick
  (params (DeltaSeconds :type Float%20%28single-precision%29)))

(fn ConstructionScript)