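; Knight enemy weapon actor that creates destruction physics fields on hits and dissolves itself with a death effect.
; CreateFields applies radial external cluster strain and linear force through its Field System at a given location, to fracture and push destructible objects.
; WeaponDissolve attaches a Niagara effect, swaps three mesh slots to a dissolve material, and runs a timeline that updates dissolve amount and emissive color through DissoleMatParam.
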(event Custom|WeaponDissolve
  (bind _dissolvematerial (Variables|Default|GetDissolveMaterial))
  (bind _itemmesh (Variables|Default|GetItemMesh))
  (Niagara|SpawnSystemAttached (Variables|Default|GetNiagaraDeathEffect) (Variables|Default|GetItemMesh) "None" "0, 0, 0" "0, 0, 0" "KeepRelativeOffset" false)
  (Utilities|FlowControl|Sequence
    (:then_0
      (Rendering|Material|SetMaterial _itemmesh 0 _dissolvematerial)
      (bind _diss (Timeline|타임라인 PlayFromStart)
        (:Update
          (CallFunction|DissoleMatParam (Variables|Default|GetItemMesh) _diss))))
    (:then_1
      (Rendering|Material|SetMaterial _itemmesh 1 _dissolvematerial)
      (Timeline|타임라인 PlayFromStart))
    (:then_2
      (Rendering|Material|SetMaterial _itemmesh 2 _dissolvematerial)
      (Timeline|타임라인 PlayFromStart))))

(event EventBeginPlay)

(event Collision|EventActorBeginOverlap
  (params (OtherActor :type Actor%20Object%20Reference)))

(event EventTick
  (params (DeltaSeconds :type Float%20%28single-precision%29)))

(event EventCreateFields
  (params (FieldLocation :type Vector%20%28by%20ref%29 :default "0, 0, 0"))
  (bind _fieldsystem (Variables|Default|GetFieldSystem))
  ;[1 1 1] 무기가 액터를 피격하였을떄 Creta Field 이벤트를 실행
  (Class|FieldSystemComponent|ApplyPhysicsField _fieldsystem true "Field_ExternalClusterStrain" 0 (Field|SetRadialFalloff (Variables|Default|GetRadialFalloff) 1e+07 0.8 1.0 0.0 2.5e+02 FieldLocation "Field_FallOff_None"))
  (Class|FieldSystemComponent|ApplyPhysicsField _fieldsystem true "Field_LinearForce" (Variables|Default|GetFieldSystemMetaDataFilter) (Field|SetRadialVector (Variables|Default|GetRadialVector) 1.5e+07 FieldLocation)))

(fn ConstructionScript)

(fn DissoleMatParam
  (params (self2 :type Mesh%20Component%20Object%20Reference) (AmountParameterValue :type Float%20%28double-precision%29))
  (Rendering|Material|SetScalarParameterValueonMaterials self2 "Dissolve" AmountParameterValue)
  (Rendering|Material|SetVectorParameterValueonMaterials self2 "Emm color" (Math|Conversions|ToVector(LinearColor) (Variables|Default|GetEffectBaseColor))))