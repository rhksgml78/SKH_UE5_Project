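; Blueprint for the Flamen undead enemy that adds a dissolve death effect on top of its parent's Die logic.
; After a delay, it attaches a Niagara effect to the mesh and swaps the first three material slots to a dissolve material.
; A timeline feeds DissoleMatParam, which animates the Dissolve scalar and sets the emissive color from EffectBaseColor.
; Tick is left empty, with the parent call disconnected.
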(event Custom|StartDeathEffect
  (bind _dissolvematerial (Variables|Default|GetDissolveMaterial))
  (bind _mesh (Variables|Character|GetMesh))
  ;[1 1 1] 사망시 호출되는 이벤트
  (Utilities|FlowControl|Delay (Variables|Default|GetDeathEffectDelay))
  (Niagara|SpawnSystemAttached (Variables|Default|GetNiagaraDeathEffect) (Variables|Character|GetMesh) "None" "0, 0, 0" "0, 0, 0" "KeepRelativeOffset" false)
  (Utilities|FlowControl|Sequence
    (:then_0
      (Rendering|Material|SetMaterial _mesh 0 _dissolvematerial)
      (bind _diss (Timeline|타임라인 PlayFromStart)
        (:Update
          (CallFunction|DissoleMatParam (Variables|Character|GetMesh) _diss))))
    (:then_1
      (Rendering|Material|SetMaterial _mesh 1 _dissolvematerial)
      (Timeline|타임라인 PlayFromStart))
    (:then_2
      (Rendering|Material|SetMaterial _mesh 2 _dissolvematerial)
      (Timeline|타임라인 PlayFromStart))))

(event EventTick
  (params (DeltaSeconds :type Float%20%28single-precision%29))
  ;[1 1 1] 매프레임 추적하려면 연결(부모연결도필수)
)

(event EventDie
  ;[1 1 1] 드래곤에게 죽으면 바로 이펙트 실행
  (|CallParentFunction)
  (CallFunction|StartDeathEffect))

(fn ConstructionScript)

(fn DissoleMatParam
  (params (self2 :type Mesh%20Component%20Object%20Reference) (AmountParameterValue :type Float%20%28double-precision%29))
  ;[1 1 1] 사망시 머테리얼의 값을 변경시키는 실행함수
  (Rendering|Material|SetScalarParameterValueonMaterials self2 "Dissolve" AmountParameterValue)
  (Rendering|Material|SetVectorParameterValueonMaterials self2 "Emm color" (Math|Conversions|ToVector(LinearColor) (Variables|Default|GetEffectBaseColor))))