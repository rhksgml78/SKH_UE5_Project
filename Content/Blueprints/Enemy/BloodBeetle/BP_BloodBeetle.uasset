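; Blood Beetle enemy Blueprint that adds a dissolve death effect on top of its parent's death logic.
; Die calls the parent, then StartDeathEffect waits a set delay and spawns an attached Niagara effect on the mesh.
; It swaps three material slots to a dissolve material and plays a timeline.
; The timeline feeds DissoleMatParam, which updates the Dissolve amount and sets the emissive color from EffectBaseColor.
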(event Custom|StartDeathEffect
  (bind _mesh (Variables|Character|GetMesh))
  (bind _dissolvematerial (Variables|Default|GetDissolveMaterial))
  ;[1 1 1] 사망시 호출되는 이벤트
  (Utilities|FlowControl|Delay (Variables|Default|GetDeathEffectDelay))
  (Niagara|SpawnSystemAttached (Variables|Default|GetNiagaraDeathEffect) (Variables|Character|GetMesh) "None" "0, 0, 0" "0, 0, 0" "KeepRelativeOffset" false)
  (Utilities|FlowControl|Sequence
    (:then_0
      (Rendering|Material|SetMaterial _mesh 0 _dissolvematerial)
      (bind _diss (Timeline|타임라인 PlayFromStart)
        (:Update
          (CallFunction|DissoleMatParam (Variables|Character|GetMesh) _diss))))
    (:then_1
      (Rendering|Material|SetMaterial _mesh 1 _dissolvematerial)
      (Timeline|타임라인 PlayFromStart))
    (:then_2
      (Rendering|Material|SetMaterial _mesh 2 _dissolvematerial)
      (Timeline|타임라인 PlayFromStart))))

(event EventBeginPlay)

(event Collision|EventActorBeginOverlap
  (params (OtherActor :type Actor%20Object%20Reference)))

(event EventTick
  (params (DeltaSeconds :type Float%20%28single-precision%29))
  (|CallParentFunction DeltaSeconds) ; 지금 이 노드는 비활성 상태입니다. \n핀을 끌어서 다른 노드를 연결하면 활성화됩니다.
)

(event EventDie
  ;[1 1 1] 드래곤에게 죽으면 바로 이펙트 실행
  (|CallParentFunction)
  (CallFunction|StartDeathEffect))

(fn ConstructionScript
  (|CallParentFunction))

(fn DissoleMatParam
  (params (self2 :type Mesh%20Component%20Object%20Reference) (AmountParameterValue :type Float%20%28double-precision%29))
  ;[1 1 1] 사망시 머테리얼의 값을 변경시키는 실행함수
  (Rendering|Material|SetScalarParameterValueonMaterials self2 "Dissolve" AmountParameterValue)
  (Rendering|Material|SetVectorParameterValueonMaterials self2 "Emm color" (Math|Conversions|ToVector(LinearColor) (Variables|Default|GetEffectBaseColor))))