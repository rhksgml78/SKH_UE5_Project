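; Dragon weapon Blueprint whose collision box kills Normal-type enemies it overlaps and spawns a Niagara fire effect at any overlapped enemy's location.
; CollisionOn and CollisionOFF set a flag, which Tick reads every frame to switch the box between query-only and no collision.
; CreateFields is an empty event, and the physics field nodes for strain and radial force are disconnected, so they never run.
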(event OnComponentBeginOverlap(DragonBoxCollision)
  (params (OverlappedComponent :type Primitive%20Component%20Object%20Reference) (OtherActor :type Actor%20Object%20Reference) (OtherComp :type Primitive%20Component%20Object%20Reference) (OtherBodyIndex :type Integer) (bFromSweep :type Boolean) (SweepResult :type Hit%20Result%20Structure%20%28by%20ref%29))
  (bind _asenemy (Utilities|Casting|CastToEnemy OtherActor))
  (if (Utilities|Enum|Equal(Enum) (Variables|/Script/SKH_UE5_Project.Enemy|GetEnemyTypes _asenemy) "ET_Normal")
    (Class|BaseCharacter|Die _asenemy))
  (Niagara|SpawnSystematLocation "/Game/EFFECT_BlinkAndDashVFX/VFX_Niagara/NS_Blink_Fire.NS_Blink_Fire" (Transformation|GetActorLocation OtherActor)))

(event Custom|CollisionOFF
  (Variables|Default|SetDragonBoxON false))

(event Custom|CollisionOn
  (Variables|Default|SetDragonBoxON true))

(event EventBeginPlay)

(event Collision|EventActorBeginOverlap
  (params (OtherActor :type Actor%20Object%20Reference)))

(event EventTick
  (params (DeltaSeconds :type Float%20%28single-precision%29))
  (if (Variables|Default|GetDragonBoxON)
    (Collision|SetCollisionEnabled (Variables|Default|GetDragonBoxCollision) "QueryOnly")
    (else
      (Collision|SetCollisionEnabled (Variables|Default|GetDragonBoxCollision) "NoCollision"))))

(event EventCreateFields
  (params (FieldLocation :type Vector%20%28by%20ref%29 :default "0, 0, 0"))
  ;[1 1 1] 무기가 액터를 피격하였을떄 Creta Field 이벤트를 실행
)

(fn ConstructionScript)