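; BP_PlayerFootSteps is an animation notify that plays surface-dependent footstep sounds and particle effects for the owning character.
; On each notify it traces the Visibility channel downward from the owner's location, ignoring the owner, and reads the hit's surface type.
; Sand, Grass and Water each spawn their own sound and effect at the impact location, while Stone shares the default branch.
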(fn ReceivedNotify
  (params (MeshComp :type Skeletal%20Mesh%20Component%20Object%20Reference) (Animation :type Anim%20Sequence%20Base%20Object%20Reference) (EventReference :type Anim%20Notify%20Event%20Reference%20Structure%20%28by%20ref%29))
  (bind _returnvalue (Components|GetOwner MeshComp))
  (bind _returnvalue_2 (Transformation|GetActorLocation _returnvalue))
  (bind (_outhit _returnvalue_3) (Collision|LineTraceByChannel _returnvalue_2 (+ _returnvalue_2 (* (Transformation|GetActorUpVector _returnvalue) -2e+02)) "TraceTypeQuery1" false (Utilities|Array|MakeArray _returnvalue) "None"))
  (if _returnvalue_3
    (switch Utilities|FlowControl|Switch|SwitchonEPhysicalSurface (Collision|GetSurfaceType _outhit)
      (:SurfaceType_Default
        (Audio|PlaySoundatLocation "/Game/SOUND_Main/MetaSounds/FootSteps/SFX_Run_Stone.SFX_Run_Stone" (.Location (Collision|BreakHitResult _outhit)) "0, 0, 0" 1.0 1.0 0.0 0 0 0 0 :!label _label)
        (Niagara|SpawnSystematLocation "/Game/A_Surface_Footstep/Niagara_FX/ParticleSystems/PSN_General1_Surface.PSN_General1_Surface" (.Location (Collision|BreakHitResult _outhit))))
      (:SurfaceType1
        (Audio|PlaySoundatLocation "/Game/SOUND_Main/MetaSounds/FootSteps/SFX_Run_Sand.SFX_Run_Sand" (.Location (Collision|BreakHitResult _outhit)) "0, 0, 0" 1.0 1.0 0.0 0 0 0 0)
        (Niagara|SpawnSystematLocation "/Game/A_Surface_Footstep/Niagara_FX/ParticleSystems/PSN_Sand_Surface.PSN_Sand_Surface" (.Location (Collision|BreakHitResult _outhit))))
      (:SurfaceType2
        (Audio|PlaySoundatLocation "/Game/SOUND_Main/MetaSounds/FootSteps/SFX_Run_Grass.SFX_Run_Grass" (.Location (Collision|BreakHitResult _outhit)) "0, 0, 0" 1.0 1.0 0.0 0 0 0 0)
        (Niagara|SpawnSystematLocation "/Game/A_Surface_Footstep/Niagara_FX/ParticleSystems/PSN_Leaves_Surface.PSN_Leaves_Surface" (.Location (Collision|BreakHitResult _outhit))))
      (:SurfaceType3
        (Audio|PlaySoundatLocation "/Game/SOUND_Main/MetaSounds/FootSteps/SFX_Run_Water.SFX_Run_Water" (.Location (Collision|BreakHitResult _outhit)) "0, 0, 0" 1.0 1.0 0.0 0 0 0 0)
        (Niagara|SpawnSystematLocation "/Game/A_Surface_Footstep/Niagara_FX/ParticleSystems/PSN_WaterLight_Surface.PSN_WaterLight_Surface" (.Location (Collision|BreakHitResult _outhit))))
      (:SurfaceType4
        (goto _label)))
    (return false)))