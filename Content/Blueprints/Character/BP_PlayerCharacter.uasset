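; Player character Blueprint that handles pause, death and overlay UI for the player, and caches BP_Unka actors as Dragon on BeginPlay.
; The pause input toggles WBP_Pause, game pause, cursor and input mode, with ClosedPausedMenu reusing the unpause path.
; DeathWidget shows and plays WBP_Death with a sound, slow motion and UI-only input.
; OverlayHideAfterShow hides the overlay, then restores it after a given delay.
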(event Custom|ClosedPausedMenu
  (bind _returnvalue (Game|GetPlayerController 0))
  (Variables|Default|SetGamePaused false)
  (Widget|RemovefromParent (stale Input|EnhancedActionEvents|EnhancedInputActionIA_PausedMenu _returnvalue_2))
  (Game|SetGamePaused false)
  (Variables|/Script/Engine.PlayerController|SetbShowMouseCursor _returnvalue false)
  (Input|SetInputModeGameOnly _returnvalue false))

(event Custom|DeathWidget
  (bind _returnvalue (Game|GetPlayerController 0))
  (bind _returnvalue_2 (UserInterface|CreateWidget "/Game/Blueprints/Widget/WBP_Death.WBP_Death_C"))
  (UserInterface|Viewport|AddtoViewport _returnvalue_2 0)
  (Default|PlayDeath _returnvalue_2)
  (Audio|PlaySound2D "/Game/SOUND_Main/OriginalSound/PlayerDeathSound.PlayerDeathSound" 1.0 1.0 0.0 0 0)
  (Utilities|Time|SetGlobalTimeDilation 0.5)
  (Variables|/Script/Engine.PlayerController|SetbShowMouseCursor _returnvalue true)
  (Input|SetInputModeUIOnly _returnvalue _returnvalue_2 "DoNotLock" false))

(event Custom|OverlayHideAfterShow
  (params (HideSecond :type Float%20%28double-precision%29))
  (Class|PlayerCharacter|HideOverlay)
  (Utilities|FlowControl|Delay HideSecond)
  (Class|PlayerCharacter|ShowOverlay))

(event Input|EnhancedActionEvents|EnhancedInputActionIA_PausedMenu
  (params (ActionValue :type Boolean) (ElapsedSeconds :type Float%20%28double-precision%29) (TriggeredSeconds :type Float%20%28double-precision%29) (InputAction :type Input%20Action%20Object%20Reference :default "/Game/Blueprints/Character/Input/IA_PausedMenu.IA_PausedMenu"))
  (bind _returnvalue (Game|GetPlayerController 0))
  (:Started
    (if (not (Variables|Default|GetGamePaused))
      (Variables|Default|SetGamePaused true)
      (bind _returnvalue_2 (UserInterface|CreateWidget "/Game/Blueprints/Widget/WBP_Pause.WBP_Pause_C"))
      (UserInterface|Viewport|AddtoViewport _returnvalue_2 0)
      (Game|SetGamePaused true)
      (Variables|/Script/Engine.PlayerController|SetbShowMouseCursor _returnvalue true)
      (Input|SetInputModeGameandUI _returnvalue _returnvalue_2 "DoNotLock" true false)
      (else
        (Variables|Default|SetGamePaused false)
        (Widget|RemovefromParent _returnvalue_2)
        (Game|SetGamePaused false)
        (Variables|/Script/Engine.PlayerController|SetbShowMouseCursor _returnvalue false)
        (Input|SetInputModeGameOnly _returnvalue false)))))

(event EventBeginPlay
  (bind _outactors (Actor|GetAllActorsOfClass "/Game/UnkaDragon/Blueprints/BP_Unka.BP_Unka_C"))
  (Variables|AllDragon|SetDragon _outactors)
  (Utilities|FlowControl|Sequence))

(event Collision|EventActorBeginOverlap
  (params (OtherActor :type Actor%20Object%20Reference)))

(event EventTick
  (params (DeltaSeconds :type Float%20%28single-precision%29)))

(fn ConstructionScript)