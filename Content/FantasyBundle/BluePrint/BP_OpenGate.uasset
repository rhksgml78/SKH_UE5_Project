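; BP_OpenGate is a double gate that opens for the player once, then shuts behind them.
; Overlap of the front trigger by BP_PlayerCharacter plays a sound and sets a flag that lets Tick swing both leaves at constant speed to yaw limits.
; Overlap of the back trigger snaps both leaves to the rotations cached at BeginPlay and permanently stops the swing, as neither flag is ever cleared.
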(event OnComponentBeginOverlap(Trigger)
  (params (OverlappedComponent :type Primitive%20Component%20Object%20Reference) (OtherActor :type Actor%20Object%20Reference) (OtherComp :type Primitive%20Component%20Object%20Reference) (OtherBodyIndex :type Integer) (bFromSweep :type Boolean) (SweepResult :type Hit%20Result%20Structure%20%28by%20ref%29))
  (Utilities|Casting|CastToBP_PlayerCharacter OtherActor)
  (if (not (Variables|Default|GetIsGateOpen))
    (Variables|Default|SetIsGateOpen true)
    (Audio|PlaySoundatLocation "/Game/SOUND_Main/MetaSounds/Enviroment/SFX_OpenGate.SFX_OpenGate" (Transformation|GetActorLocation) "0, 0, 0" 1.0 1.0 0.0 0 0 0 0)))

(event OnComponentBeginOverlap(BackTrigger)
  (params (OverlappedComponent :type Primitive%20Component%20Object%20Reference) (OtherActor :type Actor%20Object%20Reference) (OtherComp :type Primitive%20Component%20Object%20Reference) (OtherBodyIndex :type Integer) (bFromSweep :type Boolean) (SweepResult :type Hit%20Result%20Structure%20%28by%20ref%29))
  (Utilities|Casting|CastToBP_PlayerCharacter OtherActor)
  (CallFunction|ResetRotation)
  (Variables|Default|SetIsGateClose true))

(event Custom|ResetRotation
  (Transformation|SetRelativeRotation (Variables|Default|GetGateR) (Variables|Default|GetGateROrigin) false false)
  (Transformation|SetRelativeRotation (Variables|Default|GetGateL) (Variables|Default|GetGateLOrigin) false false))

(event EventBeginPlay
  (Variables|Default|SetGateROrigin (Variables|/Script/Engine.SceneComponent|GetRelativeRotation (Variables|Default|GetGateR)))
  (Variables|Default|SetGateLOrigin (Variables|/Script/Engine.SceneComponent|GetRelativeRotation (Variables|Default|GetGateL))))

(event EventTick
  (params (DeltaSeconds :type Float%20%28single-precision%29))
  (bind _gater (Variables|Default|GetGateR))
  (bind _gatel (Variables|Default|GetGateL))
  (bind _relativerotation (Variables|/Script/Engine.SceneComponent|GetRelativeRotation _gatel))
  (bind _relativerotation_2 (Variables|/Script/Engine.SceneComponent|GetRelativeRotation _gater))
  (if (and (Variables|Default|GetIsGateOpen) (not (Variables|Default|GetIsGateClose)))
    (Utilities|FlowControl|Sequence
      (:then_0
        (if (> (.yaw _relativerotation) -1.1e+02)
          (Transformation|SetRelativeRotation _gatel (Math|Rotator|MakeRotator 0.0 0.0 (- (.yaw _relativerotation) (* DeltaSeconds 2e+01))) false false)))
      (:then_1
        (if (< (.yaw _relativerotation_2) -7e+01)
          (Transformation|SetRelativeRotation _gater (Math|Rotator|MakeRotator 0.0 0.0 (+ (.yaw _relativerotation_2) (* DeltaSeconds 2e+01))) false false))))))

(fn ConstructionScript)