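; BP_ExampleAttraction is an example actor that repeatedly demonstrates the attraction portal effect from the portals VFX pack.
; It spawns and attaches a BP_Sphere_Attraction with a random portal choice, then replaces existing test cubes and skeletal-mesh actors with fresh ones randomly placed nearby.
; Tick uses a Delay to replay the BeginPlay sequence every six seconds.
; A Movement timeline that would offset the actor along Y is never run.
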(event EventBeginPlay
  (bind _returnvalue (Transformation|GetActorLocation))
  (bind _returnvalue_2 (Transformation|GetActorLocation))
  (bind _returnvalue_3 (Math|Vector|MakeVector (.x _returnvalue_2) (.y _returnvalue_2) 57.0))
  (Utilities|FlowControl|Sequence
    (:then_0
      (bind _returnvalue_4 (Game|SpawnActorfromClass "/Game/EFFECT_Portals_VFXPack/Blueprints/BP_Sphere_Attraction.BP_Sphere_Attraction_C" (Math|Transform|MakeTransform (Transformation|GetActorLocation) "0, 0, 0" "1.000000,1.000000,1.000000") "Undefined" "OverrideRootScale" 0 (Math|Random|RandomIntegerinRange 1 8) 3.0 3.0 1.5e+03 0))
      (Transformation|AttachActorToActor _returnvalue_4 self "None" "SnapToTarget" "KeepRelative" "KeepRelative" true))
    (:then_1
      (bind _outactors (Actor|GetAllActorsOfClass "/Game/EFFECT_Portals_VFXPack/Blueprints/BP_Attraction_Cube.BP_Attraction_Cube_C"))
      (for _array_element _outactors
        (Actor|DestroyActor _array_element))
      (Variables|Default|SetQuantity_Cube 0)
      (while (< (Variables|Default|GetQuantity_Cube) 3)
        (Game|SpawnActorfromClass "/Game/EFFECT_Portals_VFXPack/Blueprints/BP_Attraction_Cube.BP_Attraction_Cube_C" (Math|Transform|MakeTransform (Math|Vector|MakeVector (+ (.x _returnvalue) (Math|Random|RandomFloatinRange -7e+02 7e+02)) (+ (.y _returnvalue) (Math|Random|RandomFloatinRange -7e+02 7e+02)) (Math|Random|RandomFloatinRange 0.0 5e+01)) "0, 0, 0" "1.000000,1.000000,1.000000") "Undefined" "OverrideRootScale" 0 0)
        (Math|Integer|IncrementInt (Variables|Default|GetQuantity_Cube))))
    (:then_2
      (bind _outactors_2 (Actor|GetAllActorsOfClass "/Game/EFFECT_Portals_VFXPack/Blueprints/BP_Attraction_SkMesh.BP_Attraction_SkMesh_C"))
      (for _array_element_2 _outactors_2
        (Actor|DestroyActor _array_element_2))
      (Game|SpawnActorfromClass "/Game/EFFECT_Portals_VFXPack/Blueprints/BP_Attraction_SkMesh.BP_Attraction_SkMesh_C" (Math|Transform|MakeTransform (Math|Vector|MakeVector (+ (.x _returnvalue_3) (Math|Random|RandomFloatinRange -3e+02 3e+02)) (+ (.y _returnvalue_3) (Math|Random|RandomFloatinRange -4e+02 -1e+02)) (.z _returnvalue_3)) "0,90.000000, 0" "1.000000,1.000000,1.000000") "Undefined" "MultiplyWithRoot" 0 0)
      (Math|Integer|IncrementInt (Variables|Default|GetQuantity_SkMesh)))))

(event EventTick
  (params (DeltaSeconds :type Float%20%28single-precision%29))
  (bind _returnvalue (Transformation|GetActorLocation))
  (bind _returnvalue_2 (Transformation|GetActorLocation))
  (bind _returnvalue_3 (Math|Vector|MakeVector (.x _returnvalue_2) (.y _returnvalue_2) 57.0))
  (Utilities|FlowControl|Delay 6.0)
  (Utilities|FlowControl|Sequence
    (:then_0
      (bind _returnvalue_4 (Game|SpawnActorfromClass "/Game/EFFECT_Portals_VFXPack/Blueprints/BP_Sphere_Attraction.BP_Sphere_Attraction_C" (Math|Transform|MakeTransform (Transformation|GetActorLocation) "0, 0, 0" "1.000000,1.000000,1.000000") "Undefined" "OverrideRootScale" 0 (Math|Random|RandomIntegerinRange 1 8) 3.0 3.0 1.5e+03 0))
      (Transformation|AttachActorToActor _returnvalue_4 self "None" "SnapToTarget" "KeepRelative" "KeepRelative" true))
    (:then_1
      (bind _outactors (Actor|GetAllActorsOfClass "/Game/EFFECT_Portals_VFXPack/Blueprints/BP_Attraction_Cube.BP_Attraction_Cube_C"))
      (for _array_element _outactors
        (Actor|DestroyActor _array_element))
      (Variables|Default|SetQuantity_Cube 0)
      (while (< (Variables|Default|GetQuantity_Cube) 3)
        (Game|SpawnActorfromClass "/Game/EFFECT_Portals_VFXPack/Blueprints/BP_Attraction_Cube.BP_Attraction_Cube_C" (Math|Transform|MakeTransform (Math|Vector|MakeVector (+ (.x _returnvalue) (Math|Random|RandomFloatinRange -7e+02 7e+02)) (+ (.y _returnvalue) (Math|Random|RandomFloatinRange -7e+02 7e+02)) (Math|Random|RandomFloatinRange 0.0 5e+01)) "0, 0, 0" "1.000000,1.000000,1.000000") "Undefined" "OverrideRootScale" 0 0)
        (Math|Integer|IncrementInt (Variables|Default|GetQuantity_Cube))))
    (:then_2
      (bind _outactors_2 (Actor|GetAllActorsOfClass "/Game/EFFECT_Portals_VFXPack/Blueprints/BP_Attraction_SkMesh.BP_Attraction_SkMesh_C"))
      (for _array_element_2 _outactors_2
        (Actor|DestroyActor _array_element_2))
      (Game|SpawnActorfromClass "/Game/EFFECT_Portals_VFXPack/Blueprints/BP_Attraction_SkMesh.BP_Attraction_SkMesh_C" (Math|Transform|MakeTransform (Math|Vector|MakeVector (+ (.x _returnvalue_3) (Math|Random|RandomFloatinRange -3e+02 3e+02)) (+ (.y _returnvalue_3) (Math|Random|RandomFloatinRange -4e+02 -1e+02)) (.z _returnvalue_3)) "0,90.000000, 0" "1.000000,1.000000,1.000000") "Undefined" "MultiplyWithRoot" 0 0)
      (Math|Integer|IncrementInt (Variables|Default|GetQuantity_SkMesh)))))

(fn ConstructionScript)