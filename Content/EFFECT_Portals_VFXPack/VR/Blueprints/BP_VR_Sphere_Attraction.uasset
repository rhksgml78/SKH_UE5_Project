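; VR sphere portal effect that attracts and dissolves actors tagged PortalPack, then ends itself after a delay.
; PortalChoice selects one of eight themed Niagara looks and colors, previewed through a construction-script component.
; The gravity volume messages actors to start or stop attraction, while the inner sphere triggers a message handshake leading to dissolve.
; Shutdown reverses the size timeline, plays an end effect, spawns a decal and destroys the actor.
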(event OnComponentBeginOverlap(Sphere)
  (params (OverlappedComponent :type Primitive%20Component%20Object%20Reference) (OtherActor :type Actor%20Object%20Reference) (OtherComp :type Primitive%20Component%20Object%20Reference) (OtherBodyIndex :type Integer) (bFromSweep :type Boolean) (SweepResult :type Hit%20Result%20Structure%20%28by%20ref%29))
  ;[1 1 1] Dissolve
  (if (not (Variables|Default|GetbNoInteraction))
    (if (Actor|ActorHasTag OtherActor "PortalPack")
      (Class|BPIPortalsVfxPack|TestDissolve(Message) OtherActor self))))

(event OnComponentBeginOverlap(Gravity_Collision)
  (params (OverlappedComponent :type Primitive%20Component%20Object%20Reference) (OtherActor :type Actor%20Object%20Reference) (OtherComp :type Primitive%20Component%20Object%20Reference) (OtherBodyIndex :type Integer) (bFromSweep :type Boolean) (SweepResult :type Hit%20Result%20Structure%20%28by%20ref%29))
  ;[1 1 1] Start to attract if collision
  (if (Actor|ActorHasTag OtherActor "PortalPack")
    (Class|BPIPortalsVfxPack|GravityAttraction(Message) OtherActor self (Variables|Effectsettings|GetRadius_Attraction) (Variables|Default|GetColor) (Variables|Default|GetEffectSize))))

(event OnComponentEndOverlap(Gravity_Collision)
  (params (OverlappedComponent :type Primitive%20Component%20Object%20Reference) (OtherActor :type Actor%20Object%20Reference) (OtherComp :type Primitive%20Component%20Object%20Reference) (OtherBodyIndex :type Integer))
  ;[1 1 1] Stop the attraction
  (if (Actor|ActorHasTag OtherActor "PortalPack")
    (Class|BPIPortalsVfxPack|GravityStop(Message) OtherActor)))

(event Custom|Stop_effect
  (bind _returnvalue (Transformation|GetActorTransform))
  ;[1 1 1] Initialization
  (Utilities|FlowControl|DoOnce false
    (:Completed
      (CallFunction|StopAttraction)
      (bind _returnvalue_2 (Niagara|SpawnSystemAttached "/Game/EFFECT_Portals_VFXPack/VR/Particles/P_VR_End_Sphere.P_VR_End_Sphere" (Variables|Default|GetDefaultSceneRoot) "None" "0, 0, 0" "0, 0, 0" "KeepRelativeOffset" false))
      ;;[1 1 1] Stop the effect
      (Effects|Components|ParticleSystem|SetColorParameter _returnvalue_2 "User.Color" (Variables|Default|GetColor))
      (Effects|Components|ParticleSystem|SetColorParameter _returnvalue_2 "User.SecondaryColor" (Variables|Default|GetSecondary_Color))
      (Effects|Components|ParticleSystem|SetFloatParameter _returnvalue_2 "User.Size" (Variables|Default|GetEffectSize))
      (Utilities|FlowControl|Delay 1.0)
      (Collision|SetCollisionEnabled (Variables|Default|GetSphere) "NoCollision")
      (Components|DestroyComponent (Variables|Default|GetPortal_Effect))
      (Game|SpawnActorfromClass "/Game/EFFECT_Portals_VFXPack/Blueprints/BP_Decal.BP_Decal_C" (Math|Transform|MakeTransform (.location _returnvalue) (.rotation _returnvalue) (* (.scale _returnvalue) (* (Variables|Default|GetEffectSize) 0.4))) "Undefined" "OverrideRootScale" 0 true 0)
      (Utilities|FlowControl|Delay 1.0)
      (Actor|DestroyActor))))

(event Custom|StopAttraction
  ;[1 1 1] Effect Animation
  (bind (_direction _size _effect_size _sphere_size) (Timeline|TL_Size_Attraction Reverse)
    (:Update
      (Transformation|SetWorldScale3D (Variables|Default|GetGravity_Collision) (Math|Conversions|ToVector(Float) (* _size (Variables|Effectsettings|GetRadius_Attraction))))
      (Effects|Components|ParticleSystem|SetFloatParameter (Variables|Default|GetAttractionEffect) "User.Radius" (* _effect_size (Variables|Effectsettings|GetRadius_Attraction)))
      (Effects|Components|ParticleSystem|SetFloatParameter (Variables|Default|GetPortal_Effect) "User.SizeTeleport" (* _sphere_size (Variables|Default|GetEffectSize))))))

(event EventBeginPlay
  (bind _returnvalue (Transformation|GetActorTransform))
  (bind _attractioneffect (Variables|Default|GetAttractionEffect))
  (bind _portal_effect (Variables|Default|GetPortal_Effect))
  (bind _portal_effect_2 (Variables|Default|GetPortal_Effect))
  (bind _dissolveeffect (Variables|Default|GetDissolveEffect))
  ;[1 1 1] Initialization
  (Components|DestroyComponent (Variables|Default|GetPortalEffect_Construction))
  (Variables|Default|SetRadius (* (Variables|Default|GetRadius) (Variables|Effectsettings|GetSize)))
  (Variables|Default|SetEffectSize (/ (Variables|Effectsettings|GetSize) 4.0))
  (Transformation|SetActorRotation "90.000000,0.000000, 0")
  (switch int (Variables|Effectsettings|GetPortalChoice)
    (:1
      (Variables|Default|SetColor "(R=0.000000,G=0.548098,B=0.937500,A=1.000000)")
      (Variables|Default|SetSecondary_Color "(R=0.127180,G=0.640625,B=0.563843,A=1.000000)")
      (Class|NiagaraComponent|SetAsset _portal_effect "/Game/EFFECT_Portals_VFXPack/VR/Particles/P_VR_Electric_SpherePortal.P_VR_Electric_SpherePortal" true))
    (:2
      (Variables|Default|SetColor "(R=0.937500,G=0.182838,B=0.145520,A=1.000000)")
      (Variables|Default|SetSecondary_Color "(R=0.921875,G=0.407608,B=0.028447,A=1.000000)")
      (Class|NiagaraComponent|SetAsset _portal_effect "/Game/EFFECT_Portals_VFXPack/VR/Particles/P_VR_Fire_SpherePortal.P_VR_Fire_SpherePortal" true))
    (:3
      (Variables|Default|SetColor "(R=0.031581,G=0.796875,B=0.166799,A=1.000000)")
      (Variables|Default|SetSecondary_Color "(R=0.004161,G=0.921875,B=0.718308,A=1.000000)")
      (Class|NiagaraComponent|SetAsset _portal_effect "/Game/EFFECT_Portals_VFXPack/VR/Particles/P_VR_Natural_SpherePortal.P_VR_Natural_SpherePortal" true))
    (:4
      (Variables|Default|SetColor "(R=0.287441,G=0.412543,B=0.479320,A=1.000000)")
      (Variables|Default|SetSecondary_Color "(R=0.156168,G=0.224136,B=0.260417,A=1.000000)")
      (Class|NiagaraComponent|SetAsset _portal_effect "/Game/EFFECT_Portals_VFXPack/VR/Particles/P_VR_Fog_SpherePortal.P_VR_Fog_SpherePortal" true))
    (:5
      (Variables|Default|SetColor "(R=0.000000,G=0.548098,B=0.937500,A=1.000000)")
      (Variables|Default|SetSecondary_Color "(R=0.127180,G=0.640625,B=0.563843,A=1.000000)")
      (Class|NiagaraComponent|SetAsset _portal_effect "/Game/EFFECT_Portals_VFXPack/VR/Particles/P_VR_Ice_SpherePortal.P_VR_Ice_SpherePortal" true))
    (:6
      (Variables|Default|SetColor "(R=0.937500,G=0.518712,B=0.000000,A=1.000000)")
      (Variables|Default|SetSecondary_Color "(R=0.921875,G=0.276669,B=0.129013,A=1.000000)")
      (Class|NiagaraComponent|SetAsset _portal_effect "/Game/EFFECT_Portals_VFXPack/VR/Particles/P_VR_Light_SpherePortal.P_VR_Light_SpherePortal" true))
    (:7
      (Variables|Default|SetColor "(R=0.286492,G=0.014926,B=0.796875,A=1.000000)")
      (Variables|Default|SetSecondary_Color "(R=0.721852,G=0.019563,B=0.921875,A=1.000000)")
      (Class|NiagaraComponent|SetAsset _portal_effect "/Game/EFFECT_Portals_VFXPack/VR/Particles/P_VR_Darkness_SpherePortal.P_VR_Darkness_SpherePortal" true))
    (:8
      (Variables|Default|SetColor "(R=0.030713,G=0.473532,B=0.391573,A=1.000000)")
      (Variables|Default|SetSecondary_Color "(R=0.092728,G=0.368448,B=0.473532,A=1.000000)")
      (Class|NiagaraComponent|SetAsset _portal_effect "/Game/EFFECT_Portals_VFXPack/VR/Particles/P_VR_Futuristic_SpherePortal.P_VR_Futuristic_SpherePortal" true)))
  (Effects|Components|ParticleSystem|SetColorParameter _attractioneffect "User.Color" (Variables|Default|GetColor))
  (Effects|Components|ParticleSystem|SetColorParameter _attractioneffect "User.SecondaryColor" (Variables|Default|GetSecondary_Color))
  (Effects|Components|ParticleSystem|SetFloatParameter (Variables|Default|GetAttractionEffect) "User.Size" (Variables|Default|GetEffectSize))
  (Effects|Components|ParticleSystem|SetFloatParameter _portal_effect_2 "User.Size" (Variables|Default|GetEffectSize))
  (Effects|Components|ParticleSystem|SetFloatParameter _portal_effect_2 "User.SizeTeleport" 0.0)
  (Transformation|SetWorldScale3D (Variables|Default|GetSphere) (Math|Conversions|ToVector(Float) (* (Variables|Effectsettings|GetSize) 1.5)))
  (Effects|Components|ParticleSystem|SetFloatParameter _dissolveeffect "User.Size" (Variables|Default|GetEffectSize))
  (Effects|Components|ParticleSystem|SetColorParameter _dissolveeffect "User.Color" (Variables|Default|GetColor))
  (bind _returnvalue_2 (Niagara|SpawnSystemAttached "/Game/EFFECT_Portals_VFXPack/VR/Particles/P_VR_Sphere_Endless_Effect.P_VR_Sphere_Endless_Effect" (Variables|Default|GetDefaultSceneRoot) "None" "0, 0, 0" "0, 0, 0" "KeepRelativeOffset" true))
  (Effects|Components|ParticleSystem|SetColorParameter _returnvalue_2 "User.Color" (Variables|Default|GetColor))
  (Effects|Components|ParticleSystem|SetColorParameter _returnvalue_2 "User.SecondaryColor" (Variables|Default|GetSecondary_Color))
  (Effects|Components|ParticleSystem|SetFloatParameter _returnvalue_2 "User.Size" (Variables|Default|GetEffectSize))
  (Components|Activation|Activate (Variables|Default|GetPortal_Effect) true)
  (Utilities|FlowControl|Delay (Variables|Effectsettings|GetDelay))
  (Utilities|FlowControl|DoOnce false
    (:Completed
      (CallFunction|StopAttraction)
      (bind _returnvalue_3 (Niagara|SpawnSystemAttached "/Game/EFFECT_Portals_VFXPack/VR/Particles/P_VR_End_Sphere.P_VR_End_Sphere" (Variables|Default|GetDefaultSceneRoot) "None" "0, 0, 0" "0, 0, 0" "KeepRelativeOffset" false))
      ;;[1 1 1] Stop the effect
      (Effects|Components|ParticleSystem|SetColorParameter _returnvalue_3 "User.Color" (Variables|Default|GetColor))
      (Effects|Components|ParticleSystem|SetColorParameter _returnvalue_3 "User.SecondaryColor" (Variables|Default|GetSecondary_Color))
      (Effects|Components|ParticleSystem|SetFloatParameter _returnvalue_3 "User.Size" (Variables|Default|GetEffectSize))
      (Utilities|FlowControl|Delay 1.0)
      (Collision|SetCollisionEnabled (Variables|Default|GetSphere) "NoCollision")
      (Components|DestroyComponent (Variables|Default|GetPortal_Effect))
      (Game|SpawnActorfromClass "/Game/EFFECT_Portals_VFXPack/Blueprints/BP_Decal.BP_Decal_C" (Math|Transform|MakeTransform (.location _returnvalue) (.rotation _returnvalue) (* (.scale _returnvalue) (* (Variables|Default|GetEffectSize) 0.4))) "Undefined" "OverrideRootScale" 0 true 0)
      (Utilities|FlowControl|Delay 1.0)
      (Actor|DestroyActor))))

(event EventTestDissolve
  (params (Actor :type Actor%20Object%20Reference))
  (bind _returnvalue (Transformation|GetActorLocation Actor))
  (bind _returnvalue_2 (Transformation|GetActorLocation))
  (bind _returnvalue_3 (Math|Rotator|FindLookatRotation _returnvalue_2 _returnvalue))
  ;[1 1 1] Dissolve
  (Class|BPIPortalsVfxPack|DissolveMesh(Message) Actor (Transformation|GetWorldLocation (Variables|Default|GetSphere)) (Transformation|GetActorLocation Actor) (Variables|Default|GetColor) (/ (Variables|Effectsettings|GetSize) 4.0) (Math|Vector|GetForwardVector _returnvalue_3) (Math|Vector|GetRightVector _returnvalue_3) (Math|Vector|GetUpVector _returnvalue_3) true "None")
  (Components|Activation|Activate (Variables|Default|GetDissolveEffect) true))

(fn ConstructionScript
  (bind _portaleffect_construction (Variables|Default|GetPortalEffect_Construction))
  (bind _portaleffect_construction_2 (Variables|Default|GetPortalEffect_Construction))
  (switch int (Variables|Effectsettings|GetPortalChoice)
    (:Default
      (Class|NiagaraComponent|SetAsset _portaleffect_construction "/Game/EFFECT_Portals_VFXPack/VR/Particles/P_VR_Futuristic_SpherePortal.P_VR_Futuristic_SpherePortal" true :!label _label))
    (:0
      (Class|NiagaraComponent|SetAsset _portaleffect_construction "/Game/EFFECT_Portals_VFXPack/VR/Particles/P_VR_Electric_SpherePortal.P_VR_Electric_SpherePortal" true :!label _label_2))
    (:1
      (goto _label_2))
    (:2
      (Class|NiagaraComponent|SetAsset _portaleffect_construction "/Game/EFFECT_Portals_VFXPack/VR/Particles/P_VR_Fire_SpherePortal.P_VR_Fire_SpherePortal" true))
    (:3
      (Class|NiagaraComponent|SetAsset _portaleffect_construction "/Game/EFFECT_Portals_VFXPack/VR/Particles/P_VR_Natural_SpherePortal.P_VR_Natural_SpherePortal" true))
    (:4
      (Class|NiagaraComponent|SetAsset _portaleffect_construction "/Game/EFFECT_Portals_VFXPack/VR/Particles/P_VR_Fog_SpherePortal.P_VR_Fog_SpherePortal" true))
    (:5
      (Class|NiagaraComponent|SetAsset _portaleffect_construction "/Game/EFFECT_Portals_VFXPack/VR/Particles/P_VR_Ice_SpherePortal.P_VR_Ice_SpherePortal" true))
    (:6
      (Class|NiagaraComponent|SetAsset _portaleffect_construction "/Game/EFFECT_Portals_VFXPack/VR/Particles/P_VR_Light_SpherePortal.P_VR_Light_SpherePortal" true))
    (:7
      (Class|NiagaraComponent|SetAsset _portaleffect_construction "/Game/EFFECT_Portals_VFXPack/VR/Particles/P_VR_Darkness_SpherePortal.P_VR_Darkness_SpherePortal" true))
    (:8
      (goto _label)))
  (bind _output_get (Variables|Default|SetEffectSize (/ (Variables|Effectsettings|GetSize) 4.0)))
  (Effects|Components|ParticleSystem|SetFloatParameter _portaleffect_construction_2 "User.Size" _output_get)
  (Effects|Components|ParticleSystem|SetFloatParameter _portaleffect_construction_2 "User.SizeTeleport" _output_get)
  (Transformation|SetWorldScale3D (Variables|Default|GetSphere) (Math|Conversions|ToVector(Float) (* (Variables|Effectsettings|GetSize) 1.5))))