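; Game mode for the UnkaDragon game that respawns the player's BP_Unka character whenever it is destroyed.
; On BeginPlay it casts the player character to BP_Unka and binds to its OnDestroyed event.
; When that fires, it waits briefly, spawns a new BP_Unka at the SpawnTransform variable and has the first player controller possess it.
; It then calls Respawn to rebind the event to the new character, keeping the cycle going.
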(event Custom|OnDestroyed_Event
  (params (DestroyedActor :type Actor%20Object%20Reference))
  ;[1 1 1] Respawn
  (Utilities|FlowControl|Delay 0.2)
  (bind _returnvalue (Game|SpawnActorfromClass "/Game/UnkaDragon/Blueprints/BP_Unka.BP_Unka_C" (Variables|Default|GetSpawnTransform) "Undefined" 0 0))
  (Pawn|Possess (Game|GetPlayerController 0) _returnvalue)
  (CallFunction|Respawn))

(event Custom|Respawn
  ;[1 1 1] Respawn
  (bind _asbp_unka (Utilities|Casting|CastToBP_Unka (Game|GetPlayerCharacter 0)))
  (Game|BindEventtoOnDestroyed _asbp_unka (delegate Custom|OnDestroyed_Event)))

(event EventBeginPlay
  ;[1 1 1] Respawn
  (bind _asbp_unka (Utilities|Casting|CastToBP_Unka (Game|GetPlayerCharacter 0)))
  (Game|BindEventtoOnDestroyed _asbp_unka (delegate Custom|OnDestroyed_Event)))

(event EventTick
  (params (DeltaSeconds :type Float%20%28single-precision%29)))

(fn ConstructionScript)