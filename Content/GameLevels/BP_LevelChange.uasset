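; BP_LevelChange is an overlap trigger that moves the player between streamed levels behind a loading screen.
; When BP_PlayerCharacter overlaps it, it disables input, shows the LoadingScreen widget and blocking-loads LoadLevel.
; It then teleports the player to its Capsule's location with yaw offset 90 degrees.
; After a short delay it restores input, unloads CurrentLevel and removes the widget.
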(event EventBeginPlay)

(event Collision|EventActorBeginOverlap
  (params (OtherActor :type Actor%20Object%20Reference))
  (bind _capsule (Variables|Default|GetCapsule))
  (bind _returnvalue (Transformation|GetWorldTransform _capsule))
  (bind _asbp_player_character (Utilities|Casting|CastToBP_PlayerCharacter OtherActor))
  (bind _returnvalue_2 (UserInterface|CreateWidget (Variables|Default|GetLoadingScreen)))
  (Input|DisableInput _asbp_player_character (Game|GetPlayerController 0))
  (UserInterface|Viewport|AddtoViewport _returnvalue_2 0)
  (Class|GameplayStatics|LoadStreamLevelbySoftObjectPtr (Variables|Default|GetLoadLevel) true true)
  (Transformation|SetActorTransform _asbp_player_character (Math|Transform|MakeTransform (.location _returnvalue) (Math|Rotator|MakeRotator 0.0 0.0 (+ (.yaw (.rotation _returnvalue)) 9e+01)) "1.000000,1.000000,1.000000"))
  (Utilities|FlowControl|Delay 3.0)
  (Input|EnableInput _asbp_player_character (Game|GetPlayerController 0))
  (Class|GameplayStatics|UnloadStreamLevelbySoftObjectPtr (Variables|Default|GetCurrentLevel) true)
  (Widget|RemovefromParent _returnvalue_2))

(event EventTick
  (params (DeltaSeconds :type Float%20%28single-precision%29)))

(fn ConstructionScript)